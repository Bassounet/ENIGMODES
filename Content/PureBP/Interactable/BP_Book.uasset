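; BP_Book is an interactable book that the player grabs, with pages shown as swappable materials on its mesh.
; On first interaction it opens the WBP_Book widget, sets the player's grab flags and attaches the mesh to the spring arm.
; A timeline then lerps the mesh to the player's GrabZone location and rotation.
; NextMat and BeforeMat step through MatArray with wraparound.
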(event `/Game/PureBP/BP_InterinO.InteractMe`
  (bind _staticmesh (`self.StaticMesh`))
  (if (not (`self.Grabbed?`))
    (set `self.Grabbed?` true)
    (bind _returnvalue (`|CreateWidget` "/Game/PureBP/WIDGET/WBP_Book.WBP_Book_C"))
    (bind _output_get (set `self.Ref Widget Book` _returnvalue))
    (`UserWidget.AddToViewport` _returnvalue 0)
    (`UserWidget.AddToViewport` _output_get 0)
    (bind _asbp_first_person_character (`/Game/PureBP/BP_Function.GetPlayer`))
    (set `/Game/PureBP/Player/BP_FirstPersonCharacter.FaceOf?` true _asbp_first_person_character)
    (set `/Game/PureBP/Player/BP_FirstPersonCharacter.IsGrabbed` true _asbp_first_person_character)
    (`SceneComponent.K2_AttachToComponent` (`self.StaticMesh`) (`/Game/PureBP/Player/BP_FirstPersonCharacter.SpringArm` _asbp_first_person_character) "None" "KeepWorld" "KeepWorld" "KeepWorld" true)
    (bind (_direction _1) (`Timeline|Timeline_0` :!via `PlayFromStart`)
      (:`Update`
        (bind _grabzone (`/Game/PureBP/Player/BP_FirstPersonCharacter.GrabZone` _asbp_first_person_character))
        (`SceneComponent.K2_SetWorldLocationAndRotation` (`self.StaticMesh`) (`KismetMathLibrary.VLerp` (`SceneComponent.K2_GetComponentLocation` _staticmesh) (`SceneComponent.K2_GetComponentLocation` _grabzone) _1) (`KismetMathLibrary.RLerp` (`SceneComponent.K2_GetComponentRotation` _staticmesh) (`SceneComponent.K2_GetComponentRotation` _grabzone) _1) false false)))))

(event `NextMat`
  (bind _matarray (`self.MatArray`))
  ;[1 1 1] Mat Management
  (bind _result (`/Engine/EditorBlueprintResources/StandardMacros.IncrementFloat` (`self.Index`))
    (:`  `
      (if (not (not (>= _result (`KismetArrayLibrary.Array_Length` _matarray))))
        (set `self.Index` 0.0))
      (`PrimitiveComponent.SetMaterial` (`self.StaticMesh`) 0 (`|GetArrayItem` _matarray (`KismetMathLibrary.FTrunc` _result))))))

(event `BeforeMat`
  (bind _matarray (`self.MatArray`))
  (bind _index (`self.Index`))
  ;[1 1 1] Mat Management
  ;;[1 1 1] Mat Gest Decrement
  (if (<= _index 0.0)
    (bind _output_get (set `self.Index` (`KismetMathLibrary.Conv_IntToDouble` (- (`KismetArrayLibrary.Array_Length` _matarray) 1))))
    (`PrimitiveComponent.SetMaterial` (`self.StaticMesh`) 0 (`|GetArrayItem` _matarray (`KismetMathLibrary.FTrunc` _output_get)))
    (else
      (bind _result (`/Engine/EditorBlueprintResources/StandardMacros.DecrementFloat` _index)
        (:`  `
          (`PrimitiveComponent.SetMaterial` (`self.StaticMesh`) 0 (`|GetArrayItem` _matarray (`KismetMathLibrary.FTrunc` _result))))))))

(fn `UserConstructionScript`)