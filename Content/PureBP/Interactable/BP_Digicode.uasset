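; BP_Digicode is a keypad that builds an entered code and checks it against CodeToUnlock.
; SetDigiCode appends its input to the Code string and refreshes the CodeDisplay text.
; VerifiyCode compares the entry, prints the result to screen, then clears both Code and display.
; A correct code only prints a message; nothing is unlocked here, and the event graph is empty.
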(fn `SetDigiCode`
  (params (B :type String))
  (bind _output_get (set `self.Code` (`KismetStringLibrary.Concat_StrStr` (`self.Code`) B)))
  (`TextRenderComponent.K2_SetText` (`self.CodeDisplay`) (`KismetTextLibrary.Conv_StringToText` _output_get)))

(fn `UserConstructionScript`)

(fn `VerifiyCode`
  (bind _code (`self.Code`))
  (if (`KismetStringLibrary.EqualEqual_StrStr` _code (`self.CodeToUnlock`))
    (`KismetSystemLibrary.PrintString` (`KismetStringLibrary.Concat_StrStr` "Correct : " _code))
    (else
      (`KismetSystemLibrary.PrintString` _code)))
  (bind _output_get (set `self.Code` ""))
  (`TextRenderComponent.K2_SetText` (`self.CodeDisplay`) (`KismetTextLibrary.Conv_StringToText` _output_get)))