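; Interactable key of a digicode keypad that sends its number to the BP_Digicode actor when used.
; On BeginPlay it finds the level's BP_Digicode with GetActorOfClass and caches it along with its CodeDisplay.
; InteractMe passes the key's TouchNB value to SetDigiCode.
; The construction script writes TouchNB onto the TextRender label, so each placed key shows its own number.
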(event `self.ReceiveBeginPlay`
  (bind _returnvalue (`GameplayStatics.GetActorOfClass` "/Game/PureBP/Interactable/BP_Digicode.BP_Digicode_C"))
  (bind _output_get (set `self.Bp_Digi` _returnvalue))
  (set `self.Code Display` (`/Game/PureBP/Interactable/BP_Digicode.CodeDisplay` _output_get)))

(event `/Game/PureBP/BP_InterinO.InteractMe`
  (`/Game/PureBP/Interactable/BP_Digicode.SetDigiCode` (`self.Bp_Digi`) (`self.TouchNB`)))

(fn `UserConstructionScript`
  (`TextRenderComponent.K2_SetText` (`self.TextRender`) (`KismetTextLibrary.Conv_StringToText` (`self.TouchNB`))))