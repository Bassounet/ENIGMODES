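; BP_LaserHead is an interactable laser that, once activated, transforms a grabbable object that touches it, working only once.
; ActivateLaser shows the beam and arms the overlap check, which requires that the player is not levitating.
; On overlap it snaps the player's LevitatingObject to the head, triggers InsideLaser and a camera shake, then destroys the touching object.
; It spawns a rotating narrow-capsule grabbable at the laser and disables its own collision.
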(event `self.ReceiveBeginPlay`
  (bind _asbp_first_person_character (`/Game/PureBP/BP_Function.GetPlayer`))
  (set `self.As BP First Person Character` _asbp_first_person_character))

(event `self.StaticMesh.OnComponentBeginOverlap`
  (params (OverlappedComponent :type "PrimitiveComponent Object Reference") (OtherActor :type "Actor Object Reference") (OtherComp :type "PrimitiveComponent Object Reference") (OtherBodyIndex :type Integer) (bFromSweep :type Boolean) (SweepResult :type "HitResult Structure (by ref)"))
  (bind _as_bp_first_person_character (`self.As BP First Person Character`))
  (bind (_returnvalue_location _returnvalue_rotation) (`KismetMathLibrary.BreakTransform` (`SceneComponent.K2_GetComponentToWorld` (`self.Laser`))))
  (bind (_returnvalue_location_2 _returnvalue_rotation_2) (`KismetMathLibrary.BreakTransform` (`SceneComponent.K2_GetComponentToWorld` (`self.StaticMesh`))))
  (if (and (not (`self.Destroyed?`)) (`self.Activate?`))
    (bind _asbp_grabbable_object (cast `/Game/PureBP/Interactable/BP_GrabbableObject` OtherActor))
    (if (not (`/Game/PureBP/Player/BP_FirstPersonCharacter.levitating` _as_bp_first_person_character))
      (`SceneComponent.K2_SetWorldLocationAndRotation` (`/Game/PureBP/Player/BP_FirstPersonCharacter.levitatingObject` _as_bp_first_person_character) _returnvalue_location_2 _returnvalue_rotation_2 false false)
      (`/Game/PureBP/Interactable/BP_GrabbableObject.InsideLaser` _asbp_grabbable_object)
      (`/Game/PureBP/BP_Function.CamShakeLaserDestroy`)
      ;[0 1 0.2424] SECURE
      (`KismetSystemLibrary.Delay` 0.1)
      (`self.K2_DestroyActor` _asbp_grabbable_object)
      (bind _returnvalue (`|SpawnActorFromClass` "/Game/PureBP/Interactable/BP_GrabbableObject.BP_GrabbableObject_C" (`KismetMathLibrary.MakeTransform` _returnvalue_location _returnvalue_rotation) "AlwaysSpawn" "OverrideRootScale" null null))
      (set `self.Destroyed?` true)
      (`AddComponent|NODE_AddRotatingMovementComponent-0` :`self` _returnvalue)
      (`StaticMeshComponent.SetStaticMesh` (`/Game/PureBP/Interactable/BP_GrabbableObject.Mesh` _returnvalue) "/Game/StarterContent/Shapes/Shape_NarrowCapsule.Shape_NarrowCapsule")
      (`PrimitiveComponent.SetCollisionEnabled` (`self.StaticMesh`) "NoCollision"))))

(fn `ActivateLaser`
  (`SceneComponent.SetVisibility` (`self.Laser`) true false)
  (set `self.Activate?` true))

(fn `UserConstructionScript`)