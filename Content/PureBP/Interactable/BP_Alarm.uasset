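; BP_Alarm is an interactable alarm light that blinks until the player switches it off.
; Clignotage, started on BeginPlay, loops a timeline that lerps PointLight intensity and toggles Low each pass, though both selected targets are TargetIntensity.
; Looking at it briefly changes the MainHud cursor; interacting destroys the light and sets Destroyed to end the loop.
; BeginPlay also caches a PostProcessVolume, unused here.
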(event `/Game/PureBP/BP_InterinO.LookAtMe`
  (params (MainHud :type "/Game/PureBP/WIDGET/WBP_MainHud Object Reference"))
  (`/Game/PureBP/WIDGET/WBP_MainHud.LookingAt` MainHud (`self.In Brush Image`))
  (`KismetSystemLibrary.RetriggerableDelay` 0.03)
  (`/Game/PureBP/WIDGET/WBP_MainHud.ResetCursore` MainHud))

(event `/Game/PureBP/BP_InterinO.InteractMe`
  (`self.Switchpoint Light Off`))

(event `self.ReceiveBeginPlay`
  (`self.Clignotage`)
  (bind _returnvalue (`GameplayStatics.GetActorOfClass` "/Script/Engine.PostProcessVolume"))
  (set `self.PostProcess` _returnvalue))

(event `Clignotage`
  (`KismetSystemLibrary.RetriggerableDelay` 0.01 :!label _label)
  (if (not (`self.Destroyed?`))
    (bind (_direction _newtrack_0) (`Timeline|Timeline_0` :`NewTime` 10.0 :!via `PlayFromStart`)
      (:`Update`
        (if (not (`self.Destroyed?`))
          (`LightComponent.SetIntensity` (`self.PointLight`) (`KismetMathLibrary.Lerp` (`LightComponentBase.Intensity` (`self.PointLight`)) (`KismetMathLibrary.SelectFloat` (`self.Target Intensity +`) (`self.Target Intensity -`) (`self.Low?`)) _newtrack_0))))
      (:`Finished`
        (`TimelineComponent.SetPlayRate` (`self.Timeline_0`) (/ 1.0 (`self.Duration`)))
        (if (`self.Low?`)
          (set `self.Low?` false)
          (goto _label)
          (else
            (set `self.Low?` true)
            (goto _label)))))))

(fn `Switchpoint Light Off`
  (`ActorComponent.K2_DestroyComponent` (`self.PointLight`))
  (set `self.Destroyed?` true))

(fn `UserConstructionScript`)