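; BP_GrabbableObject is an interactable physics object that the first-person player can pick up and throw.
; InteractMe, blocked while the player's FaceOf is set, toggles between grab and release.
; Grabbing disables physics, attaches the mesh to the player's SpringArm, registers it as LevitatingObject and timeline-lerps it to GrabZone.
; Releasing, allowed only when not Levitating, detaches it, restores physics and launches it along the camera's forward vector.
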(event `self.ReceiveBeginPlay`
  (bind _asbp_first_person_character (`/Game/PureBP/BP_Function.GetPlayer`))
  (set `self.As BP First Person Character` _asbp_first_person_character))

(event `/Game/PureBP/BP_InterinO.InteractMe`
  (bind _as_bp_first_person_character (`self.As BP First Person Character`))
  (bind _as_bp_first_person_character_2 (`self.As BP First Person Character`))
  (bind _staticmesh (`self.StaticMesh`))
  (bind _grabzone (`/Game/PureBP/Player/BP_FirstPersonCharacter.GrabZone` _as_bp_first_person_character_2))
  (if (not (`/Game/PureBP/Player/BP_FirstPersonCharacter.FaceOf?` (`self.As BP First Person Character`)))
    (if (not (`self.Grabbed?`))
      (`PrimitiveComponent.SetSimulatePhysics` (`self.StaticMesh`) false)
      (set `self.Grabbed?` true)
      (set `/Game/PureBP/Player/BP_FirstPersonCharacter.levitatingObject` (`self.StaticMesh`) _as_bp_first_person_character_2)
      (`SceneComponent.K2_AttachToComponent` (`self.StaticMesh`) (`/Game/PureBP/Player/BP_FirstPersonCharacter.SpringArm` _as_bp_first_person_character_2) "None" "KeepWorld" "KeepWorld" "KeepWorld" true)
      (bind (_direction _1) (`Timeline|Timeline_0` :!via `PlayFromStart`)
        (:`Update`
          (`SceneComponent.K2_SetWorldLocationAndRotation` (`self.StaticMesh`) (`KismetMathLibrary.VLerp` (`SceneComponent.K2_GetComponentLocation` _staticmesh) (`SceneComponent.K2_GetComponentLocation` _grabzone) _1) (`KismetMathLibrary.RLerp` (`SceneComponent.K2_GetComponentRotation` _staticmesh) (`SceneComponent.K2_GetComponentRotation` _grabzone) _1) false false)))
      (elif (not (`/Game/PureBP/Player/BP_FirstPersonCharacter.levitating` (`self.As BP First Person Character`)))
        (`SceneComponent.K2_DetachFromComponent` (`self.StaticMesh`) "KeepWorld" "KeepWorld" "KeepWorld" true)
        (`PrimitiveComponent.SetSimulatePhysics` (`self.StaticMesh`) true)
        (set `self.Grabbed?` false)
        (`PrimitiveComponent.AddImpulse` (`self.StaticMesh`) (* (`SceneComponent.GetForwardVector` (`/Game/PureBP/Player/BP_FirstPersonCharacter.FirstPersonCamera` _as_bp_first_person_character)) 500.0) "None" true)
        (set `/Game/PureBP/Player/BP_FirstPersonCharacter.levitatingObject` null _as_bp_first_person_character)))))

(fn `UserConstructionScript`)