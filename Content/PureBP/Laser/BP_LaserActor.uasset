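; Laser emitter actor that traces a beam bouncing off actors tagged "Mirror" and finds the last valid actor hit.
; Rebound recursively line-traces on the Camera channel, reflecting about hit normals up to DepthLimit and storing LastValidActorHit, with trace ends not offset from their starts.
; ShootLaserMLG returns that actor, BeginPlay fires a test shot, and DebugLaser is a visualized variant.
; Debug lines, spheres and prints show each bounce.
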(event `self.ReceiveBeginPlay`
  (bind _returnvalue (`self.GetActorForwardVector`))
  (`self.Rebound` (+ _returnvalue (`self.K2_GetActorLocation`)) (* _returnvalue 100000.0) 1)
  (`KismetSystemLibrary.PrintString` "Last Hit Actor : " true true (struct :`G` 0.66 :`B` 1.0 :`A` 1.0) 10.0)
  (`KismetSystemLibrary.PrintString` (`KismetSystemLibrary.GetDisplayName` (`self.LastValidActorHit`)) true true (struct :`G` 0.66 :`B` 1.0 :`A` 1.0) 10.0))

(event `ShootLaserEvent`)

(fn `Debug Laser`
  (locals (StartToHitButWhat :type "Vector Structure"))
  (bind _returnvalue (`self.GetActorForwardVector`))
  (bind _returnvalue_2 (+ _returnvalue (`self.K2_GetActorLocation`)))
  (bind _outhit (`KismetSystemLibrary.LineTraceSingle` :`Start` _returnvalue_2 :`End` (* _returnvalue 100000.0) :`TraceChannel` "TraceTypeQuery2" :`DrawDebugType` "ForDuration" :`TraceColor` (struct :`R` 1.0 :`G` 0.145123 :`A` 1.0) :`TraceHitColor` (struct :`R` 1.0 :`G` 0.072847 :`A` 1.0) :`DrawTime` 10.0))
  (`KismetSystemLibrary.DrawDebugSphere` (`.Location` (`GameplayStatics.BreakHitResult` _outhit)) 50.0 12 (struct :`R` 1.0 :`B` 0.104708 :`A` 1.0) 10.0)
  (if (`self.ActorHasTag` (`.HitActor` (`GameplayStatics.BreakHitResult` _outhit)) "Mirror")
    (`self.Rebound` (`.Location` (`GameplayStatics.BreakHitResult` _outhit)) (`KismetMathLibrary.Normal` (`KismetMathLibrary.GetReflectionVector` (- (`.Location` (`GameplayStatics.BreakHitResult` _outhit)) _returnvalue_2) (`.Normal` (`GameplayStatics.BreakHitResult` _outhit)))) 1)))

(fn `Rebound`
  (params (StartPos :type "Vector Structure") (Direction :type "Vector Structure") (Depth :type Integer))
  (locals (StartToHit :type "Vector Structure") (HitResult :type "HitResult Structure") (LastActorHit :type "Actor Object Reference"))
  (`KismetSystemLibrary.PrintString` (`KismetStringLibrary.Conv_IntToString` Depth) true true (struct :`G` 0.66 :`B` 1.0 :`A` 1.0) 10.0)
  (bind _outhit (`KismetSystemLibrary.LineTraceSingle` :`Start` StartPos :`End` (* Direction 100000.0) :`TraceChannel` "TraceTypeQuery2" :`DrawDebugType` "ForDuration" :`TraceColor` (struct :`R` 0.874446 :`G` 1.0 :`A` 1.0) :`TraceHitColor` (struct) :`DrawTime` 10.0))
  (`KismetSystemLibrary.DrawDebugSphere` (`.Location` (`GameplayStatics.BreakHitResult` _outhit)) 35.0 12 (struct :`R` 1.0 :`G` 0.960143 :`A` 1.0) 10.0)
  (if (`KismetSystemLibrary.IsValid` (`.HitActor` (`GameplayStatics.BreakHitResult` _outhit)))
    (`KismetSystemLibrary.PrintString` (`KismetSystemLibrary.GetDisplayName` (`.HitActor` (`GameplayStatics.BreakHitResult` _outhit))) true true (struct :`R` 0.186399 :`B` 1.0 :`A` 1.0) 10.0)
    (bind _output_get (set `self.LastValidActorHit` (`.HitActor` (`GameplayStatics.BreakHitResult` _outhit))))
    (if (`self.ActorHasTag` _output_get "Mirror")
      (if (< Depth (`self.DepthLimit`))
        (bind _result (`/Engine/EditorBlueprintResources/StandardMacros.IncrementInt` Depth)
          (:`  `
            (`self.Rebound` (`.Location` (`GameplayStatics.BreakHitResult` _outhit)) (`KismetMathLibrary.Normal` (`KismetMathLibrary.GetReflectionVector` (- (`.Location` (`GameplayStatics.BreakHitResult` _outhit)) StartPos) (`.Normal` (`GameplayStatics.BreakHitResult` _outhit)))) _result)))
        (else
          (`KismetSystemLibrary.PrintString` "Depth limit reached, returning the last valid object hit" true true (struct :`G` 1.0 :`B` 0.002892 :`A` 1.0) 10.0)
          (`KismetSystemLibrary.PrintString` (`KismetSystemLibrary.GetDisplayName` (`self.LastValidActorHit`)) true true (struct :`R` 0.19512 :`G` 1.0 :`A` 1.0) 10.0 :!label _label)
          (return)))
      (else
        (`KismetSystemLibrary.PrintString` "Actor Hit isn't a Mirror, returning the last obj" true true (struct :`G` 0.080408 :`B` 1.0 :`A` 1.0) 10.0)
        (goto _label)))
    (else
      (`KismetSystemLibrary.PrintString` "Last Actor Hit Not Valid, returning the previous one if there is one" true true (struct :`R` 1.0 :`B` 0.026276 :`A` 1.0) 10.0)
      (if (`KismetSystemLibrary.IsValid` (`self.LastValidActorHit`))
        (return)
        (else
          (`KismetSystemLibrary.PrintString` "Not valid actor, returning nullptr" true true (struct :`R` 1.0 :`G` 0.035352 :`A` 1.0) 10.0)
          (return))))))

(fn `ShootLaserMLG`
  (returns (ActorHit :type "Actor Object Reference"))
  (bind _returnvalue (`self.GetActorForwardVector`))
  (`self.Rebound` (+ _returnvalue (`self.K2_GetActorLocation`)) (* _returnvalue 100000.0) 1)
  (return (`self.LastValidActorHit`)))

(fn `UserConstructionScript`)